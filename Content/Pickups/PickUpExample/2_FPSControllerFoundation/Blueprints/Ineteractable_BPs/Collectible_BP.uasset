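; Collectible pickup actor that spins and bobs in place until the player collects it.
; Tick adds yaw rotation each frame and plays the Bob timeline, whose vector track is applied as a local offset.
; When the player pawn overlaps it, it plays a 2D sound, spawns a particle effect at its Sphere component and destroys itself.
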(event `self.ReceiveActorBeginOverlap`
  (params (OtherActor :type "Actor Object Reference"))
  (if (== OtherActor (`GameplayStatics.GetPlayerPawn` 0))
    (`GameplayStatics.PlaySound2D` null)
    (`GameplayStatics.SpawnEmitterAtLocation` null (`SceneComponent.K2_GetComponentLocation` (`self.Sphere`)))
    (`self.K2_DestroyActor`)))

(event `self.ReceiveTick`
  (params (DeltaSeconds :type "Float (single-precision)"))
  (`self.K2_AddActorLocalRotation` (struct :`Yaw` 3.0))
  (bind (_direction _newtrack_0) (`Timeline|Bob`)
    (:`Update`
      (`self.K2_AddActorLocalOffset` _newtrack_0))))

(fn `UserConstructionScript`)