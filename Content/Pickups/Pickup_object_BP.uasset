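; Scrap pickup that homes in on the player and awards scrap to the robot character when it arrives.
; Overlapping its Box with RobotCharacter_BP1 sets PickedUp, after which Tick runs RotateAndSeek and grows SpeedTimer.
; Each frame it steps toward player 0 by SpeedTimer times CollectSpeed, accelerating without delta-time scaling, while SetActorLocationAndRotation overwrites the preceding local spin.
; Within a small distance it calls DestroyActor, then CollectScrap on the player.
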(event `self.ReceiveTick`
  (params (DeltaSeconds :type "Float (single-precision)"))
  (set `self.DeltaTime` DeltaSeconds)
  (set `self.PlayerPosition` (`self.GetTransform` (`GameplayStatics.GetPlayerPawn` 0)))
  (if (`self.PickedUp`)
    (`self.RotateAndSeek`)
    (set `self.SpeedTimer` (+ (`self.DeltaTime`) (`self.SpeedTimer`)))))

(event `self.ReceiveBeginPlay`
  (set `self.StartPosition` (`self.GetTransform`)))

(event `self.Box.OnComponentBeginOverlap`
  (params (OverlappedComponent :type "PrimitiveComponent Object Reference") (OtherActor :type "Actor Object Reference") (OtherComp :type "PrimitiveComponent Object Reference") (OtherBodyIndex :type Integer) (bFromSweep :type Boolean) (SweepResult :type "HitResult Structure (by ref)"))
  (cast `/Game/RobotCharacter/RobotCharacter_BP1` OtherActor)
  (set `self.PickedUp` true))

(fn `RotateAndSeek`
  (bind _rotationspeed (`self.RotationSpeed`))
  (bind _returnvalue (* (`KismetMathLibrary.MakeRotator` _rotationspeed _rotationspeed _rotationspeed) (`self.DeltaTime`)))
  (if (< (`self.GetDistanceTo` (`GameplayStatics.GetPlayerPawn` 0)) 3.0)
    (`self.K2_DestroyActor`)
    (bind _asrobot_character_bp1 (cast `/Game/RobotCharacter/RobotCharacter_BP1` (`GameplayStatics.GetPlayerPawn` 0)))
    (`/Game/RobotCharacter/RobotCharacter_BP1.CollectScrap` _asrobot_character_bp1 (`self.Scrap`))
    (else
      (`self.K2_AddActorLocalRotation` _returnvalue)
      (`self.K2_SetActorLocationAndRotation` (+ (* (`KismetMathLibrary.GetDirectionUnitVector` (.location (`self.GetTransform`)) (.location (`self.PlayerPosition`))) (* (`self.SpeedTimer`) (`self.CollectSpeed`))) (.location (`self.GetTransform`))) _returnvalue))))

(fn `UserConstructionScript`)